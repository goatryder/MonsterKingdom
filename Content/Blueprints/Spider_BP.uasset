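; Spider enemy Blueprint that drives a world-space health bar widget.
; On BeginPlay it caches the player character, hands itself to the Enemy_Health_UI widget and binds to its enemy hit delegate.
; Critical hits trigger the widget's crit effect.
; Every Tick rotates the widget component to face the player's follow camera, billboard style.
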(event Custom|EnemyHitDelegate_Event_0
  (params (HitDamage :type Float%20%28single-precision%29) (CritHit :type Boolean))
  ;[1 1 1] Bind Event To Enemy Get Attack
  (if CritHit
    (Default|CritEnemyWidgetEffect (Variables|Default|GetHealthWidgetREF))))

(event EventBeginPlay
  ;[1 1 1] Get Player REF
  (bind _asmain_character_bp (Utilities|Casting|CastToMainCharacter_BP (Game|GetPlayerCharacter 0)))
  (Variables|Default|SetPlayerREF _asmain_character_bp)
  ;[1 1 1] Setup Health Bar
  (bind _asenemy_health_ui (Utilities|Casting|CastToEnemy_Health_UI (UserInterface|GetUserWidgetObject (Variables|Default|GetWidget))))
  (Variables|Default|SetHealthWidgetREF _asenemy_health_ui)
  (Variables|/Game/UI/Enemy_Health_UI.Enemy_Health_UI_C|SetEnemyREF _asenemy_health_ui self)
  ;[1 1 1] Bind Event To Enemy Get Attack
  (EventDispatchers|AssignEnemyHitDelegate (delegate Custom|EnemyHitDelegate_Event_0)))

(event EventTick
  (params (DeltaSeconds :type Float%20%28single-precision%29))
  (bind _scene_widget (Variables|Default|GetScene%20Widget))
  (bind _playerref (Variables|Default|GetPlayerREF))
  (bind _returnvalue (Transformation|GetWorldLocation _scene_widget))
  (bind _followcamera (Variables|/Script/MonsterKingdom.MainCharacter|GetFollowCamera _playerref))
  (bind _returnvalue_2 (Transformation|GetWorldLocation _followcamera))
  (bind _returnvalue_3 (Math|Rotator|FindLookatRotation _returnvalue _returnvalue_2))
  (Transformation|SetWorldRotation (Variables|Default|GetWidget) (Math|Rotator|MakeRotator (.roll _returnvalue_3) (.pitch _returnvalue_3) (.yaw _returnvalue_3)) false false))

(fn ConstructionScript)